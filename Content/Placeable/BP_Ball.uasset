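; BP_Ball is a placeable physics ball whose mesh comes from the DT_Balls data table, looked up by its Name.
; On BeginPlay it applies the mesh, enables physics and overlaps, moves the actor just above the level's BP_Plane, then calls InitPos.
; InitPos lifts the mesh above the actor, adjusts location and rotation by its Root socket, and zeroes its linear and angular velocity.
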(event EventBeginPlay
  (bind _staticmesh (Variables|Default|GetStaticMesh))
  (bind _returnvalue (Utilities|GetDataTableRow "/Game/Placeable/Balls/DT_Balls.DT_Balls" (Variables|Default|GetName))
    (:then
      (Components|StaticMesh|SetStaticMesh (Variables|Default|GetStaticMesh) (.Mesh (Utilities|Struct|BreakST_Balls _returnvalue)))
      (Physics|SetSimulatePhysics _staticmesh true)
      (Variables|/Script/Engine.PrimitiveComponent|SetbGenerateOverlapEvents _staticmesh true)
      (bind _returnvalue_2 (Actor|GetActorOfClass "/Game/Placeable/BP_Plane.BP_Plane_C"))
      (Transformation|SetActorLocation (+ (Transformation|GetActorLocation _returnvalue_2) "0.000000,0.000000,10.000000") false false)
      (CallFunction|InitPos))))

(fn ConstructionScript)

(fn InitPos
  (bind _staticmesh (Variables|Default|GetStaticMesh))
  (bind _staticmesh_2 (Variables|Default|GetStaticMesh))
  (bind _returnvalue (Transformation|GetSocketTransform _staticmesh "Root" "RTS_ParentBoneSpace"))
  (Transformation|SetWorldLocation (Variables|Default|GetStaticMesh) (+ (Transformation|GetActorLocation) "0.000000,0.000000,200.000000") false false)
  (Transformation|AddRelativeLocation _staticmesh (* (.location _returnvalue) -1.0) false false)
  (Transformation|SetRelativeRotation (Variables|Default|GetStaticMesh) (.rotation _returnvalue) false false)
  (Class|PrimitiveComponent|SetPhysicsAngularVelocityinDegrees _staticmesh_2 "0, 0, 0" false "None")
  (Physics|SetPhysicsLinearVelocity _staticmesh_2 "0, 0, 0" false "None"))