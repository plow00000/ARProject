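; BP_Goalpost is a placeable goal that returns a BP_Ball to its initial position when the ball overlaps its center component.
; On BeginPlay it finds the BP_Plane actor and attaches to that plane's floor, keeping world scale.
; It then sits just inside one edge of the plane's box, using the IsWidthLonger flag to pick the X or Y axis and rotating 90 degrees for Y.
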(event OnComponentBeginOverlap(goalpost_center)
  (params (OverlappedComponent :type Primitive%20Component%20Object%20Reference) (OtherActor :type Actor%20Object%20Reference) (OtherComp :type Primitive%20Component%20Object%20Reference) (OtherBodyIndex :type Integer) (bFromSweep :type Boolean) (SweepResult :type Hit%20Result%20Structure%20%28by%20ref%29))
  (bind _asbp_ball (Utilities|Casting|CastToBP_Ball OtherActor))
  (Default|InitPos _asbp_ball))

(event EventBeginPlay
  (bind _returnvalue (Actor|GetActorOfClass "/Game/Placeable/BP_Plane.BP_Plane_C"))
  (Transformation|AttachComponentToComponent (Variables|/Game/Placeable/BP_Plane.BP_Plane_C|GetFloor _returnvalue) "None" "KeepRelative" "KeepRelative" "KeepWorld" true)
  (Transformation|SetActorRelativeLocation "0, 0, 0")
  (if (Variables|/Game/Placeable/BP_Plane.BP_Plane_C|GetbIsWidthLonger _returnvalue)
    (Transformation|SetActorRelativeLocation (Math|Vector|MakeVector (- (.x (Components|Box|GetUnscaledBoxExtent (Variables|/Game/Placeable/BP_Plane.BP_Plane_C|GetBox _returnvalue))) 1e+01) 0.0 0.0))
    (else
      (Transformation|SetActorRelativeLocation (Math|Vector|MakeVector 0.0 (- (.y (Components|Box|GetUnscaledBoxExtent (Variables|/Game/Placeable/BP_Plane.BP_Plane_C|GetBox _returnvalue))) 1e+01) 0.0))
      (Transformation|SetActorRelativeRotation "0.000000,90.000000,0.000000"))))

(fn ConstructionScript)