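; AR player controller that scans for a floor plane to host the court, with a main widget whose Rescan button restarts scanning.
; Tick periodically traces tracked geometry at screen center, replacing BP_Plane until CheckSize yields a valid court size, then broadcasts PlaneSpawned.
; For test-level use, left-click traces world objects to place planes without broadcasting.
; Temporary mouse and movement inputs drive the pawn, and V substitutes for the confirm button.
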(event Custom|Rescan
  (Variables|Default|SetbIsScanDone false))

(event Input|EnhancedActionEvents|EnhancedInputActionIA_Move
  (params (ActionValue :type Vector%202D%20Structure) (ElapsedSeconds :type Float%20%28double-precision%29) (TriggeredSeconds :type Float%20%28double-precision%29) (InputAction :type Input%20Action%20Object%20Reference :default "/Game/IA_Move.IA_Move"))
  (bind _returnvalue (Utilities|Time|GetWorldDeltaSeconds))
  (bind _returnvalue_2 (* ActionValue _returnvalue 1e+03))
  (bind (_x _y) (Math|Vector2D|BreakVector2D _returnvalue_2))
  ;[0.15 0.15 0.15 0.5] Lvl_Test에서 사용할 용도
  ;;[0.15 0.15 0.15 0.5] 폰 조작(임시)
  (Transformation|AddActorLocalOffset (Pawn|GetControlledPawn) (Math|Vector|MakeVector _x _y 0.0) false false))

(event EventBeginPlay
  ;[0.15 0.15 0.15 0.5] Test 레벨 사용시 위쪽, Main 레벨 사용시 아래 쪽
  (bind _returnvalue (UserInterface|CreateWidget "/Game/UI/MainWidget.MainWidget_C" self))
  (bind _output_get (Variables|Default|SetWidget _returnvalue))
  (UserInterface|Viewport|AddtoViewport _output_get 0)
  (EventDispatchers|BindEventtoOnClicked (Variables|/Game/UI/MainWidget.MainWidget_C|GetRescanButton (Variables|Default|GetWidget)) (delegate Custom|Rescan)))

(event EventTick
  (params (DeltaSeconds :type Float%20%28single-precision%29))
  ;[0.15 0.15 0.15 0.5] Test 레벨에서는 끊기
  (if (not (Variables|Default|GetbIsScanDone))
    (bind _output_get (Variables|Default|SetShowPlaneTime (+ (Variables|Default|GetShowPlaneTime) DeltaSeconds)))
    (if (> _output_get 1.0)
      (CallFunction|UpdatePlaneCandidated))))

(event Input|MouseEvents|LeftMouseButton
  (params (Key :type Key%20Structure :default "None"))
  ;[0.15 0.15 0.15 0.5] Lvl_Test에서 사용할 용도
  ;;[0.15 0.15 0.15 0.5] 좌클릭 시 플레인 생성 시도
  (:Pressed
    (CallFunction|UpdatePlaneTest)))

(event Input|KeyboardEvents|V
  (params (Key :type Key%20Structure :default "None"))
  (bind _self self)
  ;[0.15 0.15 0.15 0.5] Lvl_Test에서 사용할 용도
  ;;[0.15 0.15 0.15 0.5] 결정 버튼 대신 해주려고 V키 할당
  (:Pressed
    (bind _asbp_argame_state (Utilities|Casting|CastToBP_ARGameState (Game|GetGameState)))
    (Default|ChangeState _asbp_argame_state "NewEnumerator8")
    (Input|SetInputModeGameandUI _self 0 "DoNotLock" true false)
    (Variables|Default|SetbShowMouseCursor _self true)))

(event Input|MouseEvents|Mouse2D
  (params (AxisValue :type Vector :default "0, 0, 0"))
  ;[0.15 0.15 0.15 0.5] Lvl_Test에서 사용할 용도
  ;;[0.15 0.15 0.15 0.5] 카메라 회전(임시)
  (bind _asbp_arpawn (Utilities|Casting|CastToBP_ARPawn (Pawn|GetControlledPawn)))
  (Transformation|AddRelativeRotation (Variables|/Game/GameFrameWork/BP_ARPawn.BP_ARPawn_C|GetCamera _asbp_arpawn) (Math|Rotator|MakeRotator 0.0 (.y AxisValue) (.x AxisValue)) false false))

(fn ConstructionScript)

(fn UpdatePlaneCandidated
  (bind _returnvalue (Class|ARBlueprintLibrary|LineTraceTrackedObjects (* (Viewport|GetViewportSize) 0.5)))
  (if (Math|Conversions|ToBoolean(Integer) (Utilities|Array|Length _returnvalue))
    (bind _asarplane_geometry (Utilities|Casting|CastToARPlaneGeometry (Class|ARTraceResultLibrary|GetTrackedGeometry (Utilities|Array|Get(acopy) _returnvalue))))
    (bind _returnvalue_2 (Game|SpawnActorfromClass "/Game/Placeable/BP_Plane.BP_Plane_C" (Class|ARTrackedGeometry|GetLocaltoWorldTransform _asarplane_geometry) "Undefined" "MultiplyWithRoot" 0 0))
    (Transformation|SetRelativeScale3D (Variables|/Game/Placeable/BP_Plane.BP_Plane_C|GetFloor _returnvalue_2) (Math|Vector|MakeVector (.x (/ (Class|ARPlaneGeometry|GetExtent _asarplane_geometry) 5e+01)) (.y (/ (Class|ARPlaneGeometry|GetExtent _asarplane_geometry) 5e+01)) 1.0))
    (Utilities|FlowControl|Sequence
      (:then_0
        (bind _plane (Variables|Default|GetPlane)
          (:then
            (Actor|DestroyActor _plane))
          (:else)))
      (:then_1
        (bind _output_get (Variables|Default|SetPlane _returnvalue_2))
        (Default|CheckSize _output_get)
        (Variables|Default|SetShowPlaneTime 0.0)
        (if (Math|Conversions|ToBoolean(Integer) (Variables|/Game/Placeable/BP_Plane.BP_Plane_C|GetSizeOfCourt (Variables|Default|GetPlane)))
          (Variables|Default|SetbIsScanDone true)
          (Default|CallDispatcherPlaneSpawned))))))

(fn UpdatePlaneTest
  (bind (_locationx _locationy) (Game|Player|GetMousePosition))
  (bind _self self)
  (bind (_worldposition _worlddirection) (Class|GameplayStatics|DeprojectScreentoWorld _self (Math|Vector2D|MakeVector2D _locationx _locationy)))
  (bind _asbp_argame_state (Utilities|Casting|CastToBP_ARGameState (Game|GetGameState)))
  (if (Utilities|Enum|Equal(Enum) (Variables|/Game/GameFrameWork/BP_ARGameState.BP_ARGameState_C|GetCurrentState _asbp_argame_state) "NewEnumerator0")
    (bind (_outhit _returnvalue) (Collision|LineTraceForObjects _worldposition (+ _worldposition (* _worlddirection 1e+03)) (Utilities|Array|MakeArray "ObjectTypeQuery2") false 0 "None"))
    (if _returnvalue
      (bind _returnvalue_2 (Game|SpawnActorfromClass "/Game/Placeable/BP_Plane.BP_Plane_C" (Transformation|GetActorTransform (.HitActor (Collision|BreakHitResult _outhit))) "Undefined" "MultiplyWithRoot" 0 0))
      (Transformation|SetRelativeScale3D (Variables|/Game/Placeable/BP_Plane.BP_Plane_C|GetFloor _returnvalue_2) (Math|Vector|MakeVector (.x (/ (.Scale (Math|Transform|BreakTransform (Transformation|GetActorTransform (.HitActor (Collision|BreakHitResult _outhit))))) 0.25)) (.y (/ (.Scale (Math|Transform|BreakTransform (Transformation|GetActorTransform (.HitActor (Collision|BreakHitResult _outhit))))) 0.25)) (.z (/ (.Scale (Math|Transform|BreakTransform (Transformation|GetActorTransform (.HitActor (Collision|BreakHitResult _outhit))))) 0.25))))
      (Utilities|FlowControl|Sequence
        (:then_0
          (bind _plane (Variables|Default|GetPlane)
            (:then
              (Actor|DestroyActor _plane))
            (:else)))
        (:then_1
          (bind _output_get (Variables|Default|SetPlane _returnvalue_2))
          (Transformation|AddActorLocalOffset _output_get "0.000000,0.000000,1.000000" false false)
          (Default|CheckSize _output_get)
          (Variables|Default|SetShowPlaneTime 0.0)
          (Variables|Default|SetbIsScanDone true))))))